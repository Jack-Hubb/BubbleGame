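; Bubble machine actor that provides a shrinking breathable zone, which an interaction event grows back.
; Tick steadily reduces the radius, resizing the guide sphere and scaling the Bubble through a clamped range map.
; Bubble overlaps stop or start the overlapping actor's suffocation message.
; When the player's Sphere1 crosses the boundary, it also switches volumetric fog start distance and toggles the level's post-process volume, off inside and on outside.
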(event `self.ReceiveBeginPlay`
  (bind _asbp_main_player_character (cast `/Game/Blueprints/Player/BP_MainPlayerCharacter` (`GameplayStatics.GetPlayerCharacter` 0)))
  (set `self.playerRef` _asbp_main_player_character)
  (bind _returnvalue (`GameplayStatics.GetActorOfClass` "/Script/Engine.ExponentialHeightFog"))
  (set `self.fogRef` _returnvalue)
  (bind _returnvalue_2 (`GameplayStatics.GetActorOfClass` "/Script/Engine.PostProcessVolume"))
  (set `self.postProcess` _returnvalue_2))

(event `self.ReceiveTick`
  (params (DeltaSeconds :type "Float (single-precision)"))
  (bind _currentbubbleradius (`self.currentBubbleRadius`))
  (`SphereComponent.SetSphereRadius` (`self.BubbleGuide`) _currentbubbleradius true)
  (`SceneComponent.SetWorldScale3D` (`self.Bubble`) (`KismetMathLibrary.Conv_DoubleToVector` (`KismetMathLibrary.MapRangeClamped` _currentbubbleradius 0.0 (`self.maxBubbleRadius`) 0.0 800.0)))
  (set `self.currentBubbleRadius` (- (`self.currentBubbleRadius`) DeltaSeconds (`self.scaleVariable`))))

(event `self.growBubbleInteraction`
  (`self.growBubble` 200.0))

(event `self.Bubble.OnComponentBeginOverlap`
  (params (OverlappedComponent :type "PrimitiveComponent Object Reference") (OtherActor :type "Actor Object Reference") (OtherComp :type "PrimitiveComponent Object Reference") (OtherBodyIndex :type Integer) (bFromSweep :type Boolean) (SweepResult :type "HitResult Structure (by ref)"))
  ; Player Enters Bubble
  (message `/Game/Blueprints/BPI/BPI_PlayerBubbleInteractions.stopSuffocation` OtherActor)
  (if (== OtherComp (`/Game/Blueprints/Player/BP_MainPlayerCharacter.Sphere1` (`self.playerRef`)))
    (`ExponentialHeightFogComponent.SetVolumetricFogStartDistance` (`ExponentialHeightFog.Component` (`self.fogRef`)) 2000.0)
    (set `PostProcessVolume.bEnabled` false (`self.postProcess`))))

(event `self.Bubble.OnComponentEndOverlap`
  (params (OverlappedComponent :type "PrimitiveComponent Object Reference") (OtherActor :type "Actor Object Reference") (OtherComp :type "PrimitiveComponent Object Reference") (OtherBodyIndex :type Integer))
  (message `/Game/Blueprints/BPI/BPI_PlayerBubbleInteractions.startSuffocation` OtherActor)
  (if (== OtherComp (`/Game/Blueprints/Player/BP_MainPlayerCharacter.Sphere1` (`self.playerRef`)))
    (`ExponentialHeightFogComponent.SetVolumetricFogStartDistance` (`ExponentialHeightFog.Component` (`self.fogRef`)) 500.0)
    (set `PostProcessVolume.bEnabled` true (`self.postProcess`))))

(fn `growBubble`
  (params (growAmount :type "Float (double-precision)"))
  (set `self.currentBubbleRadius` (+ (`self.currentBubbleRadius`) growAmount)))

(fn `UserConstructionScript`
  (`SphereComponent.SetSphereRadius` (`self.BubbleGuide`) (`self.currentBubbleRadius`) true))