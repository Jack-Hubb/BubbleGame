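; BP_Submarine is a world object that collects four repair parts from the player and then opens the main cutscene level.
; On interact within range, it scans the player's inventory for gear, wing, module and window item IDs, removes them and sets matching flags.
; Tick polls those flags and triggers the level load once through a DoOnce when all are set.
; A sphere overlap shows and hides a widget.
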(event `self.ReceiveBeginPlay`
  (`self.EnableInput` (`GameplayStatics.GetPlayerController` 0))
  (bind _asbp_main_player_character (cast `/Game/Blueprints/Player/BP_MainPlayerCharacter` (`GameplayStatics.GetPlayerCharacter` 0)))
  (set `self.playerRef` _asbp_main_player_character))

(event `EnhancedInput|/Game/Blueprints/Game/Input/InputActions/IA_Interact`
  (params (ActionValue :type Boolean) (ElapsedSeconds :type "Float (double-precision)") (TriggeredSeconds :type "Float (double-precision)") (InputAction :type "InputAction Object Reference" :default "/Game/Blueprints/Game/Input/InputActions/IA_Interact.IA_Interact"))
  (bind _inventory (`/Game/Blueprints/Components/BPC_Inventory.inventory` (`/Game/Blueprints/Player/BP_MainPlayerCharacter.inventoryComponentRef` (`self.playerRef`))))
  (:`Completed`
    (if (< (`KismetMathLibrary.Vector_Distance` (`self.K2_GetActorLocation`) (`self.K2_GetActorLocation` (`GameplayStatics.GetPlayerCharacter` 0))) 500.0)
      (for _array_element _inventory
        (if (== _array_element 1)
          (set `self.hasGear` true)
          (`KismetSystemLibrary.PrintString` "submit gear")
          (`KismetArrayLibrary.Array_RemoveItem` _inventory 1)
          (elif (== _array_element 2)
            (set `self.hasWing` true)
            (`KismetSystemLibrary.PrintString` "submit wing")
            (`KismetArrayLibrary.Array_RemoveItem` _inventory 2)
            (elif (== _array_element 3)
              (set `self.hasModule` true)
              (`KismetSystemLibrary.PrintString` "submit module")
              (`KismetArrayLibrary.Array_RemoveItem` _inventory 3)
              (elif (== _array_element 5)
                (set `self.hasWindow` true)
                (`KismetSystemLibrary.PrintString` "submit window")
                (`KismetArrayLibrary.Array_RemoveItem` _inventory 5)))))))))

(event `self.ReceiveTick`
  (params (DeltaSeconds :type "Float (single-precision)"))
  (if (and (`self.hasGear`) (`self.hasModule`) (`self.hasWing`) (`self.hasWindow`))
    (`/Engine/EditorBlueprintResources/StandardMacros.DoOnce` false
      (:`Completed`
        (`GameplayStatics.OpenLevelBySoftObjectPtr` "/Game/Levels/L_Main_cutscene.L_Main_cutscene")))))

(event `self.Sphere.OnComponentBeginOverlap`
  (params (OverlappedComponent :type "PrimitiveComponent Object Reference") (OtherActor :type "Actor Object Reference") (OtherComp :type "PrimitiveComponent Object Reference") (OtherBodyIndex :type Integer) (bFromSweep :type Boolean) (SweepResult :type "HitResult Structure (by ref)"))
  (`SceneComponent.SetHiddenInGame` (`self.Widget`) false false))

(event `self.Sphere.OnComponentEndOverlap`
  (params (OverlappedComponent :type "PrimitiveComponent Object Reference") (OtherActor :type "Actor Object Reference") (OtherComp :type "PrimitiveComponent Object Reference") (OtherBodyIndex :type Integer))
  (`SceneComponent.SetHiddenInGame` (`self.Widget`) true false))

(fn `getPlayerRef`
  (returns (playerRef :type "/Game/Blueprints/Player/BP_MainPlayerCharacter Object Reference"))
  (return null))

(fn `UserConstructionScript`)