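; BPC_Inventory is an inventory component that stores item IDs in an array, with zero marking an empty slot.
; CollectItem treats the inventory as full when the slot at index 3 is occupied, returning true without storing the item.
; Otherwise it loops through the array, writes the ID into the first empty slot and stops.
; The event graph holds only disabled placeholder events.
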(fn `collectItem`
  (params (itemID :type Integer))
  (returns (isFull :type Boolean))
  (if (!= (`|GetArrayItem` (`self.inventory`) 3) 0)
    (return true)
    (else
      (for (_array_element _array_index) (`self.inventory`)
        (if (== _array_element 0)
          (`KismetArrayLibrary.Array_Set` (`self.inventory`) _array_index itemID)
          (break))))))