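; BP_Pickup is a ground item that hovers in the world and can be collected by the player.
; The construction script sets its mesh and material from DT_Items, using ItemID minus one as the row index.
; Sphere overlap by the player passes ItemID to the inventory component's CollectItem, destroying the pickup with a sound when that returns false.
; Either result closes the gate that drives the Tick-based hover timeline.
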(event `self.ReceiveBeginPlay`)

(event `self.ReceiveTick`
  (params (DeltaSeconds :type "Float (single-precision)"))
  (`/Engine/EditorBlueprintResources/StandardMacros.Gate` false :!label _label
    (:`Exit`
      (bind (_direction _hover) (`Timeline|Hover`)
        (:`Update`
          (`SceneComponent.K2_AddWorldOffset` (`self.Cube`) (`KismetMathLibrary.MakeVector` 0.0 0.0 _hover) false false))))))

(event `self.Sphere.OnComponentBeginOverlap`
  (params (OverlappedComponent :type "PrimitiveComponent Object Reference") (OtherActor :type "Actor Object Reference") (OtherComp :type "PrimitiveComponent Object Reference") (OtherBodyIndex :type Integer) (bFromSweep :type Boolean) (SweepResult :type "HitResult Structure (by ref)"))
  (bind _returnvalue (`GameplayStatics.GetPlayerCharacter` 0))
  (if (== OtherActor _returnvalue)
    (bind _playerref (message `/Game/Blueprints/BPI/BPI_Player.getPlayerRef` _returnvalue))
    (bind _isfull (`/Game/Blueprints/Components/BPC_Inventory.CollectItem` (`/Game/Blueprints/Player/BP_MainPlayerCharacter.inventoryComponentRef` _playerref) (`self.itemID`)))
    (if _isfull
      (goto _label :!via `Close`)
      (else
        (`self.K2_DestroyActor`)
        (`GameplayStatics.PlaySoundAtLocation` "/Game/Sound/SFX/PickUpMetal.PickUpMetal" (`self.K2_GetActorLocation`) (struct) 1.0 1.0 0.0 null null null null)
        (goto _label :!via `Close`)))))

(fn `UserConstructionScript`
  (bind _cube (`self.Cube`))
  ; TODO: change mesh based on item lookup in datatable
  (bind _outrownames (`DataTableFunctionLibrary.GetDataTableRowNames` "/Game/Blueprints/DataTables/DT_Items.DT_Items"))
  (bind _returnvalue (`|GetDataTableRow` "/Game/Blueprints/DataTables/DT_Items.DT_Items" (`|GetArrayItem` _outrownames (- (`self.itemID`) 1)))
    (:`then`
      (`StaticMeshComponent.SetStaticMesh` _cube (`.Mesh_13_9CEA459445DB015CD3500BA404B11618` (break `/Game/Blueprints/DataTables/S_Items` _returnvalue)))
      (`PrimitiveComponent.SetMaterial` _cube 0 (`.Material_16_1A6C5C474C435657AD5946B40ACEAF66` (break `/Game/Blueprints/DataTables/S_Items` _returnvalue))))))