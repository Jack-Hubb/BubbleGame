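; Bubble machine ground item that maintains a safe bubble, which shrinks every tick and grows through a GrowBubbleInteraction event.
; Tick syncs the guide sphere and bubble mesh to the current radius, while a timeline animates the tube, handle and burst effects.
; Player overlaps toggle suffocation messages, fog start distance and post-process.
; A hidden trigger launches the player forward and upward as secret movement tech.
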(event `self.ReceiveBeginPlay`
  (`|ExecutionSequence`
    (:`then_0`
      (bind (_direction _newtrack_0) (`Timeline|Timeline`)
        (:`Update`
          (`SceneComponent.SetWorldScale3D` (`self.TubeThing`) (`KismetMathLibrary.MakeVector` 0.5 0.5 _newtrack_0))
          (`/Engine/EditorBlueprintResources/StandardMacros.IncrementFloat` (`self.rot`)
            (:`  `
              (`SceneComponent.K2_SetWorldRotation` (`self.Handle`) (`KismetMathLibrary.MakeRotator` 0.0 0.0 (`self.rot`)) false false))))
        (:`BubbleEventTrack`
          (`NiagaraFunctionLibrary.SpawnSystemAtLocation` "/Game/Art/Particles/NS_BubbleBurst.NS_BubbleBurst" (`SceneComponent.K2_GetComponentLocation` (`self.BubbleBurst`)) (struct) (0.5 0.5 0.5)))))
    (:`then_1`
      (bind _asbp_main_player_character (cast `/Game/Blueprints/Player/BP_MainPlayerCharacter` (`GameplayStatics.GetPlayerCharacter` 0)))
      (set `self.playerRef` _asbp_main_player_character)
      (bind _returnvalue (`GameplayStatics.GetActorOfClass` "/Script/Engine.ExponentialHeightFog"))
      (set `self.fogRef` _returnvalue))))

(event `self.ReceiveTick`
  (params (DeltaSeconds :type "Float (single-precision)"))
  (bind _currentbubbleradius (`self.currentBubbleRadius`))
  (`SphereComponent.SetSphereRadius` (`self.BubbleGuide`) _currentbubbleradius true)
  (`SceneComponent.SetWorldScale3D` (`self.Bubble`) (`KismetMathLibrary.Conv_DoubleToVector` (`KismetMathLibrary.MapRangeClamped` _currentbubbleradius 0.0 (`self.maxBubbleRadius`) 0.0 800.0)))
  (set `self.currentBubbleRadius` (- (`self.currentBubbleRadius`) DeltaSeconds (`self.scaleVariable`))))

(event `/Game/Blueprints/BPI/BPI_PlayerBubbleInteractions.growBubbleInteraction`
  (`self.growBubble` 100.0))

(event `self.Bubble.OnComponentBeginOverlap`
  (params (OverlappedComponent :type "PrimitiveComponent Object Reference") (OtherActor :type "Actor Object Reference") (OtherComp :type "PrimitiveComponent Object Reference") (OtherBodyIndex :type Integer) (bFromSweep :type Boolean) (SweepResult :type "HitResult Structure (by ref)"))
  (if (== OtherActor (`GameplayStatics.GetPlayerCharacter` 0))
    (message `/Game/Blueprints/BPI/BPI_PlayerBubbleInteractions.stopSuffocation` OtherActor)
    (if (== OtherComp (`/Game/Blueprints/Player/BP_MainPlayerCharacter.Sphere1` (`self.playerRef`)))
      (`ExponentialHeightFogComponent.SetVolumetricFogStartDistance` (`ExponentialHeightFog.Component` (`self.fogRef`)) 2000.0)
      (set `PostProcessComponent.bEnabled` false (`/Game/Blueprints/Player/BP_MainPlayerCharacter.PostProcess` (`self.playerRef`))))))

(event `self.Bubble.OnComponentEndOverlap`
  (params (OverlappedComponent :type "PrimitiveComponent Object Reference") (OtherActor :type "Actor Object Reference") (OtherComp :type "PrimitiveComponent Object Reference") (OtherBodyIndex :type Integer))
  (if (== OtherActor (`GameplayStatics.GetPlayerCharacter` 0))
    (message `/Game/Blueprints/BPI/BPI_PlayerBubbleInteractions.startSuffocation` OtherActor)
    (if (== OtherComp (`/Game/Blueprints/Player/BP_MainPlayerCharacter.Sphere1` (`self.playerRef`)))
      (`ExponentialHeightFogComponent.SetVolumetricFogStartDistance` (`ExponentialHeightFog.Component` (`self.fogRef`)) 500.0)
      (set `PostProcessComponent.bEnabled` true (`/Game/Blueprints/Player/BP_MainPlayerCharacter.PostProcess` (`self.playerRef`))))))

(event `self.shhhh secret.OnComponentBeginOverlap`
  (params (OverlappedComponent :type "PrimitiveComponent Object Reference") (OtherActor :type "Actor Object Reference") (OtherComp :type "PrimitiveComponent Object Reference") (OtherBodyIndex :type Integer) (bFromSweep :type Boolean) (SweepResult :type "HitResult Structure (by ref)"))
  ; the sacred movement tech
  (bind _asbp_main_player_character (cast `/Game/Blueprints/Player/BP_MainPlayerCharacter` OtherActor))
  (bind (_returnvalue_x _returnvalue_y) (`KismetMathLibrary.BreakVector` (* (`self.GetActorForwardVector` _asbp_main_player_character) 2500.0)))
  (`Character.LaunchCharacter` _asbp_main_player_character (`KismetMathLibrary.MakeVector` _returnvalue_x _returnvalue_y 1900.0) false false))

(fn `growBubble`
  (params (growAmount :type "Float (double-precision)"))
  (set `self.currentBubbleRadius` (+ (`self.currentBubbleRadius`) growAmount)))

(fn `UserConstructionScript`
  (bind _currentbubbleradius (`self.currentBubbleRadius`))
  (`SphereComponent.SetSphereRadius` (`self.BubbleGuide`) _currentbubbleradius true)
  (`SceneComponent.SetWorldScale3D` (`self.Bubble`) (`KismetMathLibrary.Conv_DoubleToVector` (`KismetMathLibrary.MapRangeClamped` _currentbubbleradius 0.0 (`self.maxBubbleRadius`) 0.0 800.0))))