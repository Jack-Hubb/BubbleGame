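; BP_BubbleSpawner is a spawner actor that scatters BP_Bubble actors across a large area at a timed rate.
; On BeginPlay it passes itself to the player character and starts a looping timer at SpawnRate.
; Each tick of that timer, while under a fixed cap, runs a slanted random top-to-bottom line trace and spawns at the hit location without checking for a hit.
; GetBubble decrements the count, freeing room for more.
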(event `self.ReceiveBeginPlay`
  (message `/Game/Blueprints/BPI/BPI_PlayerBubbleInteractions.BubbleMakerRef` (`GameplayStatics.GetPlayerCharacter` 0) self)
  (`KismetSystemLibrary.K2_SetTimerDelegate` (delegate `CustomEvent`) (`self.spawnRate`) true))

(event `CustomEvent`
  (bind _returnvalue (`KismetMathLibrary.RandomFloatInRange` -25000.0 25000.0))
  (bind _returnvalue_2 (`KismetMathLibrary.RandomFloatInRange` -25000.0 25000.0))
  (if (< (`self.currentBubbles`) 150)
    (bind _outhit (`KismetSystemLibrary.LineTraceSingle` (`KismetMathLibrary.MakeVector` _returnvalue_2 _returnvalue 9999.0) (`KismetMathLibrary.MakeVector` _returnvalue_2 _returnvalue -9999.0) "TraceTypeQuery1"))
    (`|SpawnActorFromClass` "/Game/Blueprints/GroundItems/BP_Bubble.BP_Bubble_C" (`KismetMathLibrary.MakeTransform` (`KismetMathLibrary.MakeVector` (.x (`.Location` (`GameplayStatics.BreakHitResult` _outhit))) (.y (`.Location` (`GameplayStatics.BreakHitResult` _outhit))) (.z (`.Location` (`GameplayStatics.BreakHitResult` _outhit))))) "Undefined" "MultiplyWithRoot" null 0 null)
    (`/Engine/EditorBlueprintResources/StandardMacros.IncrementInt` (`self.currentBubbles`))))

(event `/Game/Blueprints/BPI/BPI_PlayerBubbleInteractions.getBubble`
  (`/Engine/EditorBlueprintResources/StandardMacros.DecrementInt` (`self.currentBubbles`)))

(fn `UserConstructionScript`)