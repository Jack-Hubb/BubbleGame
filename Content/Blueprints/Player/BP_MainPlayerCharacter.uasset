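; Main player character for an underwater bubble-and-shark game, handling input, HUD, pause menu, inventory and health.
; BeginPlay applies GameInstance distortion, border and film-grain settings through post-processing.
; Suffocation events drain and refill air with Delay loops, apply drowning damage, and death resets health and teleports to world origin.
; Held bubbles grow the main bubble, while Tick flags shooed AI via blackboard and drives danger music from shark distance.
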(event `EnhancedInput|/Game/Blueprints/Game/Input/InputActions/IA_Pause`
  (params (ActionValue :type Boolean) (ElapsedSeconds :type "Float (double-precision)") (TriggeredSeconds :type "Float (double-precision)") (InputAction :type "InputAction Object Reference" :default "/Game/Blueprints/Game/Input/InputActions/IA_Pause.IA_Pause"))
  (bind _returnvalue (`GameplayStatics.GetPlayerController` 0))
  (:`Completed`
    (bind _returnvalue_2 (`|CreateWidget` "/Game/Blueprints/UI/WBP_Pause.WBP_Pause_C"))
    (`UserWidget.AddToViewport` _returnvalue_2 0)
    (bind _output_get (set `PlayerController.bShowMouseCursor` true _returnvalue))
    (`WidgetBlueprintLibrary.SetInputMode_UIOnlyEx` _returnvalue null)
    ;[0.15 0.15 0.15 0.5 32] Apply Graphics Settings
    ;; Wave Strength
    (`GameplayStatics.SetGamePaused` _output_get)))

(event `self.ReceiveBeginPlay`
  (set `self.health` (`self.maxHealth`))
  (set `self.maxRemainingAir` (`self.remainingAir`))
  (bind _returnvalue (`|CreateWidget` "/Game/Blueprints/UI/WD_HUD.WD_HUD_C"))
  (`UserWidget.AddToViewport` _returnvalue 0)
  (bind _returnvalue_2 (`AddComponent|NODE_AddBPC_Inventory-7` :`owningPlayer` self))
  (set `self.inventoryComponentRef` _returnvalue_2)
  (`|ExecutionSequence`
    (:`then_0`
      (bind _asgi_game_instance (cast `/Game/Blueprints/Game/GI_GameInstance` (`GameplayStatics.GetGameInstance`)))
      (set `self.gameInstanceRef` _asgi_game_instance))
    (:`then_1`
      ;[0.15 0.15 0.15 0.5 32] Apply Graphics Settings
      (bind _returnvalue_3 (`KismetMaterialLibrary.CreateDynamicMaterialInstance` "/Game/Art/Materials/M_PostProcess.M_PostProcess"))
      (`|ExecutionSequence`
        (:`then_0`
          ;; Wave Strength
          (switch `int` (`/Game/Blueprints/Game/GI_GameInstance.waterDistortionSetting` (`self.gameInstanceRef`))
            (:`0`
              (`MaterialInstanceDynamic.SetScalarParameterValue` _returnvalue_3 "Wave Strength" 0.0))
            (:`1`
              (`MaterialInstanceDynamic.SetScalarParameterValue` _returnvalue_3 "Wave Strength" 0.01))
            (:`2`
              (`MaterialInstanceDynamic.SetScalarParameterValue` _returnvalue_3 "Wave Strength" 0.03))
            (:`3`
              (`MaterialInstanceDynamic.SetScalarParameterValue` _returnvalue_3 "Wave Strength" 0.05))
            (:`4`
              (`MaterialInstanceDynamic.SetScalarParameterValue` _returnvalue_3 "Wave Strength" 0.1))))
        (:`then_1`
          ;; Border
          (if (`/Game/Blueprints/Game/GI_GameInstance.borderSetting` (`self.gameInstanceRef`))
            (`MaterialInstanceDynamic.SetScalarParameterValue` _returnvalue_3 "Border Strength" 0.3)
            (else
              (`MaterialInstanceDynamic.SetScalarParameterValue` _returnvalue_3 "Border Strength" 0.0))))
        (:`then_2`
          (if (`/Game/Blueprints/Game/GI_GameInstance.filmGrain` (`self.gameInstanceRef`))
            (set `PostProcessComponent.Settings` (make `PostProcessSettings` :`FilmBlackClip` 0.03 :`SceneFringeIntensity` 2.036001 :`BloomIntensity` 2.978999 :`FilmGrainIntensity` 0.5 :`FilmGrainIntensityShadows` 0.43 :`FilmGrainIntensityMidtones` 0.6 :`FilmGrainIntensityHighlights` 0.28 :`FilmGrainTexelSize` 0.76 :`DepthOfFieldSensorWidth` 250.0 :`DepthOfFieldFocalDistance` 400.0) (`self.PostProcess`))
            (else
              (set `PostProcessComponent.Settings` (make `PostProcessSettings` :`FilmBlackClip` 0.03 :`SceneFringeIntensity` 2.036001 :`BloomIntensity` 2.978999 :`DepthOfFieldSensorWidth` 250.0 :`DepthOfFieldFocalDistance` 400.0) (`self.PostProcess`)))))
        (:`then_3`
          (`PostProcessComponent.AddOrUpdateBlendable` (`self.PostProcess`) _returnvalue_3 1.0))))
    (:`then_2`
      (bind _outactors (`GameplayStatics.GetAllActorsOfClass` "/Game/Blueprints/Enemies/Shark/BP_Shark.BP_Shark_C"))
      (set `self.sharks` _outactors))))

(event `EnhancedInput|/Game/Blueprints/Game/Input/InputActions/IA_Movement`
  (params (ActionValue :type "Vector2D Structure") (ElapsedSeconds :type "Float (double-precision)") (TriggeredSeconds :type "Float (double-precision)") (InputAction :type "InputAction Object Reference" :default "/Game/Blueprints/Game/Input/InputActions/IA_Movement.IA_Movement"))
  (bind _walkspeed (`self.walkSpeed`))
  ; Input
  ;; Movement
  (:`Triggered`
    (`self.AddMovementInput` (`self.GetActorForwardVector`) (* ActionValue_Y _walkspeed))
    (`self.AddMovementInput` (`self.GetActorRightVector`) (* ActionValue_X _walkspeed)))
  (:`Started`
    (set `self.isWalking` true))
  (:`Completed`
    (set `self.isWalking` false)))

(event `EnhancedInput|/Game/Blueprints/Game/Input/InputActions/IA_Jump`
  (params (ActionValue :type Boolean) (ElapsedSeconds :type "Float (double-precision)") (TriggeredSeconds :type "Float (double-precision)") (InputAction :type "InputAction Object Reference" :default "/Game/Blueprints/Game/Input/InputActions/IA_Jump.IA_Jump"))
  ; Input
  (:`Started`
    (set `self.jumpStarted` true)
    (`self.Jump`)
    (`KismetSystemLibrary.Delay` 0.2)
    (set `self.jumpStarted` false)))

(event `EnhancedInput|/Game/Blueprints/Game/Input/InputActions/IA_Look`
  (params (ActionValue :type "Vector2D Structure") (ElapsedSeconds :type "Float (double-precision)") (TriggeredSeconds :type "Float (double-precision)") (InputAction :type "InputAction Object Reference" :default "/Game/Blueprints/Game/Input/InputActions/IA_Look.IA_Look"))
  ; Input
  (:`Triggered`
    (`self.AddControllerYawInput` (* ActionValue_X 1.0))
    (`self.AddControllerPitchInput` (* ActionValue_Y -1.0))))

(event `EnhancedInput|/Game/Blueprints/Game/Input/InputActions/IA_Interact`
  (params (ActionValue :type Boolean) (ElapsedSeconds :type "Float (double-precision)") (TriggeredSeconds :type "Float (double-precision)") (InputAction :type "InputAction Object Reference" :default "/Game/Blueprints/Game/Input/InputActions/IA_Interact.IA_Interact"))
  ; Grow Main Bubble
  (:`Completed`
    (if (and (> (`self.heldBubbles`) 0) (not (`self.suffocating`)))
      (`/Engine/EditorBlueprintResources/StandardMacros.DecrementInt` (`self.heldBubbles`)
        (:`  `
          (message `/Game/Blueprints/BPI/BPI_PlayerBubbleInteractions.growBubbleInteraction` (stale `self.interactionCollider.OnComponentBeginOverlap` OtherActor)))))))

(event `self.interactionCollider.OnComponentBeginOverlap`
  (params (OverlappedComponent :type "PrimitiveComponent Object Reference") (OtherActor :type "Actor Object Reference") (OtherComp :type "PrimitiveComponent Object Reference") (OtherBodyIndex :type Integer) (bFromSweep :type Boolean) (SweepResult :type "HitResult Structure (by ref)"))
  ; Grow Main Bubble
)

(event `/Game/Blueprints/BPI/BPI_PlayerBubbleInteractions.startSuffocation`
  (bind _remainingair (`self.remainingAir`))
  ; Suffication
  (set `self.suffocating` true)
  (bind _returnvalue (`GameplayStatics.SpawnSound2D` "/Game/Sound/SFX/UnderWaterAmbience.UnderWaterAmbience" 1.0 1.0 0.0 null))
  (bind _output_get (set `self.ambience` _returnvalue))
  (`AudioComponent.FadeIn` _output_get 1.0 1.0 0.0 "Linear")
  (if (<= _remainingair 0.0) :!label _label
    (`KismetSystemLibrary.K2_SetTimerDelegate` (delegate `Suffocate`) 1.5 :!label _label_2)
    (else
      (`/Engine/EditorBlueprintResources/StandardMacros.DecrementFloat` _remainingair
        (:`  `
          (`KismetSystemLibrary.Delay` 0.2)
          (if (`self.suffocating`)
            (goto _label)))))))

(event `Suffocate`
  ; Suffication
  (if (`self.suffocating`)
    (`ActorComponent.Activate` (`self.Drowning`) false)
    (if (<= 0.0 (`self.health`))
      (set `self.health` (- (`self.health`) 4.0))
      (goto _label_2)
      (else
        (`GameplayStatics.PlaySound2D` "/Game/Sound/SFX/DeathScream.DeathScream" 1.0 1.0 0.0 null null)
        (`self.KillPlayer`)))
    (else
      (`ActorComponent.Deactivate` (`self.Drowning`)))))

(event `/Game/Blueprints/BPI/BPI_PlayerBubbleInteractions.stopSuffocation`
  (bind _ambience (`self.ambience`))
  ; Suffication
  (set `self.suffocating` false)
  (`/Engine/EditorBlueprintResources/StandardMacros.IsValid` _ambience
    (:`Is Valid`
      (`AudioComponent.FadeOut` _ambience 1.0 0.0 "Linear")
      (`ActorComponent.K2_DestroyComponent` _ambience))
    (:`Is Not Valid`
      _))
  (if (< (`self.remainingAir`) (`self.maxRemainingAir`)) :!label _label_3
    (`/Engine/EditorBlueprintResources/StandardMacros.IncrementFloat` (`self.remainingAir`)
      (:`  `
        (`KismetSystemLibrary.Delay` 0.1)
        (goto _label_3)))))

(event `KillPlayer`
  ; TODO : RESPAWN PLAYER AND RESET INVENTORY
  (set `self.health` (`self.maxHealth`))
  (`self.K2_SetActorLocation` self (0.0 0.0 0.0) false false))

(event `self.ReceiveAnyDamage`
  (params (Damage :type "Float (single-precision)") (DamageType :type "DamageType Object Reference") (InstigatedBy :type "Controller Object Reference") (DamageCauser :type "Actor Object Reference"))
  (set `self.health` (- (`self.health`) Damage)))

(event `EnhancedInput|/Game/Blueprints/Game/Input/InputActions/IA_Emote`
  (params (ActionValue :type Boolean) (ElapsedSeconds :type "Float (double-precision)") (TriggeredSeconds :type "Float (double-precision)") (InputAction :type "InputAction Object Reference" :default "/Game/Blueprints/Game/Input/InputActions/IA_Emote.IA_Emote"))
  (:`Started`
    (set `self.emoting` true)
    (`KismetSystemLibrary.Delay` 0.2)
    (set `self.emoting` false)))

(event `/Game/Blueprints/BPI/BPI_PlayerBubbleInteractions.BubbleMakerRef`
  (params (BubbleMakerRef :type "/Game/Blueprints/GroundItems/BP_BubbleSpawner Object Reference"))
  (set `self.Bubble Maker Ref` BubbleMakerRef))

(event `/Game/Blueprints/BPI/BPI_PlayerBubbleInteractions.getBubble`
  (message `/Game/Blueprints/BPI/BPI_PlayerBubbleInteractions.getBubble` (`self.Bubble Maker Ref`))
  (`/Engine/EditorBlueprintResources/StandardMacros.IncrementInt` (`self.heldBubbles`)))

(event `/Game/Blueprints/BPI/BPI_EnemyInteractions.Knockback`
  (params (hitImpulse :type "Vector Structure"))
  (`self.LaunchCharacter` hitImpulse))

(event `self.Sphere.OnComponentEndOverlap`
  (params (OverlappedComponent :type "PrimitiveComponent Object Reference") (OtherActor :type "Actor Object Reference") (OtherComp :type "PrimitiveComponent Object Reference") (OtherBodyIndex :type Integer))
  (set `self.inShooingRange` false))

(event `self.Sphere.OnComponentBeginOverlap`
  (params (OverlappedComponent :type "PrimitiveComponent Object Reference") (OtherActor :type "Actor Object Reference") (OtherComp :type "PrimitiveComponent Object Reference") (OtherBodyIndex :type Integer) (bFromSweep :type Boolean) (SweepResult :type "HitResult Structure (by ref)"))
  (set `self.inShooingRange` true))

(event `EnhancedInput|/Game/Blueprints/Game/Input/InputActions/IA_Shoo`
  (params (ActionValue :type Boolean) (ElapsedSeconds :type "Float (double-precision)") (TriggeredSeconds :type "Float (double-precision)") (InputAction :type "InputAction Object Reference" :default "/Game/Blueprints/Game/Input/InputActions/IA_Shoo.IA_Shoo"))
  (:`Triggered`
    (set `self.isShooing` true)
    (`KismetSystemLibrary.Delay` 4.0)
    (set `self.isShooing` false)))

(event `self.ReceiveTick`
  (params (DeltaSeconds :type "Float (single-precision)"))
  (bind _sharks (`self.sharks`))
  (`|ExecutionSequence`
    (:`then_0`
      (if (<= (`self.health`) 0.0)
        (`self.KillPlayer`)
        (elif (and (`self.isShooing`) (`self.inShooingRange`))
          (`BlackboardComponent.SetValueAsBool` (`AIBlueprintHelperLibrary.GetBlackboard` (`AIBlueprintHelperLibrary.GetAIController` (stale `self.Sphere.OnComponentBeginOverlap` OtherActor))) "beingShood" true))))
    (:`then_1`
      (for _array_element _sharks
        (if (<= (`self.GetDistanceTo` _array_element) 4000.0)
          (`self.SharkChaseBegin`)
          (else
            (`/Engine/EditorBlueprintResources/StandardMacros.IncrementInt` (`self.sharkOutOfRangeCounter`)))))
      (if (== (`KismetArrayLibrary.Array_Length` _sharks) (`self.sharkOutOfRangeCounter`))
        (set `self.sharkOutOfRangeCounter` 0)
        (`/Engine/EditorBlueprintResources/StandardMacros.IsValid` (stale `SharkChaseBegin` _returnvalue)
          (:`Is Valid`
            (`AudioComponent.FadeOut` (stale `SharkChaseBegin` _returnvalue) 1.0 0.0 "Linear")
            (`ActorComponent.K2_DestroyComponent` (stale `SharkChaseBegin` _returnvalue))
            (goto _label_4 :!via `Reset`)))
        (else
          (set `self.sharkOutOfRangeCounter` 0))))))

(event `SharkChaseBegin`
  (`/Engine/EditorBlueprintResources/StandardMacros.DoOnce` false :!label _label_4
    (:`Completed`
      (bind _returnvalue (`GameplayStatics.SpawnSound2D` "/Game/Sound/Music/SW_Music_DangerClose.SW_Music_DangerClose" 1.0 1.0 0.0 null)))))

(fn `getPlayerRef`
  (returns (playerRef :type "/Game/Blueprints/Player/BP_MainPlayerCharacter Object Reference"))
  (return self))

(fn `UserConstructionScript`)