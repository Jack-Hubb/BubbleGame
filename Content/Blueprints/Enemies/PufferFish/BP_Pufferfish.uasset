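; Pufferfish enemy that spots pawns, and knocks back and damages actors that touch it.
; A timeline started on BeginPlay animates the mesh's relative Z position.
; PawnSensing writes the seen pawn and a seePlayer flag to the AI blackboard, and Tick clears the flag once the player is beyond a set distance.
; Sphere overlap sends a knockback message along the mesh's forward vector and applies damage.
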(event `self.ReceiveBeginPlay`
  (bind (_direction _vectortrack) (`Timeline|Timeline`)
    (:`Update`
      (`SceneComponent.K2_SetRelativeLocation` (`self.Mesh`) (`KismetMathLibrary.MakeVector` 0.0 0.0 (.z _vectortrack)) false false))))

(event `self.PawnSensing.OnSeePawn`
  (params (Pawn :type "Pawn Object Reference"))
  (bind _returnvalue (`AIBlueprintHelperLibrary.GetBlackboard` (`AIBlueprintHelperLibrary.GetAIController` self)))
  (`/Engine/EditorBlueprintResources/StandardMacros.IsValid` Pawn
    (:`Is Valid`
      (`BlackboardComponent.SetValueAsObject` _returnvalue "PlayerRef" Pawn)
      (`BlackboardComponent.SetValueAsBool` _returnvalue "seePlayer" true))))

(event `self.ReceiveTick`
  (params (DeltaSeconds :type "Float (single-precision)"))
  (if (> (`KismetMathLibrary.Vector_Distance` (`self.K2_GetActorLocation` (`GameplayStatics.GetPlayerCharacter` 0)) (`self.K2_GetActorLocation`)) 2800.0)
    (`BlackboardComponent.SetValueAsBool` (`AIBlueprintHelperLibrary.GetBlackboard` (`AIBlueprintHelperLibrary.GetAIController` self)) "seePlayer" false)))

(event `self.Sphere.OnComponentBeginOverlap`
  (params (OverlappedComponent :type "PrimitiveComponent Object Reference") (OtherActor :type "Actor Object Reference") (OtherComp :type "PrimitiveComponent Object Reference") (OtherBodyIndex :type Integer) (bFromSweep :type Boolean) (SweepResult :type "HitResult Structure (by ref)"))
  (message `/Game/Blueprints/BPI/BPI_EnemyInteractions.Knockback` OtherActor (* (`SceneComponent.GetForwardVector` (`self.Mesh`)) 2000.0))
  (`GameplayStatics.ApplyDamage` OtherActor 15.0))

(fn `UserConstructionScript`)